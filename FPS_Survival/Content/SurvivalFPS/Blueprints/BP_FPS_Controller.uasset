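; BP_FPS_Controller is a first-person character Blueprint that adds head bob to the player's camera.
; Every tick, a Headbob event checks velocity and CanJump, then starts a Walk or Sprint camera shake by speed threshold while moving and able to jump.
; Otherwise it starts the Idle shake, so standing still and being unable to jump share the same motion.
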(event Custom|Headbob
  (bind _returnvalue (Transformation|GetVelocity))
  (bind _returnvalue_2 (Game|GetPlayerController 0))
  (bind _returnvalue_3 (Math|Vector|VectorLength _returnvalue))
  ;[1 1 1] Headbob
  (if (and (> _returnvalue_3 0.0) (Character|CanJump))
    (if (< _returnvalue_3 3e+02)
      (Game|Feedback|ClientStartCameraShake _returnvalue_2 "/Game/SurvivalFPS/HeadBob/Walk.Walk_C" 1.0 "CameraLocal" "0, 0, 0")
      (else
        (Game|Feedback|ClientStartCameraShake _returnvalue_2 "/Game/SurvivalFPS/HeadBob/Sprint.Sprint_C" 1.0 "CameraLocal" "0, 0, 0")))
    (else
      (Game|Feedback|ClientStartCameraShake _returnvalue_2 "/Game/SurvivalFPS/HeadBob/idle.idle_C" 1.0 "CameraLocal" "0, 0, 0"))))

(event EventBeginPlay)

(event Collision|EventActorBeginOverlap
  (params (OtherActor :type Actor%20Object%20Reference)))

(event EventTick
  (params (DeltaSeconds :type Float%20%28single-precision%29))
  ;[1 1 1] Headbob
  (CallFunction|Headbob))

(fn ConstructionScript)